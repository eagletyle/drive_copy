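; Time trial manager that runs a lap race over an ordered list of checkpoints.
; On BeginPlay it passes lap count, save slot and default best times to MainPlayerController, then numbers the checkpoints and binds their cleared events.
; Each clear reveals and enables the next checkpoint and moves the respawn point to the cleared one.
; The last checkpoint updates the lap, looping to the first or flagging the race complete and restarting through the controller.
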(event Custom|Apply%20Settings
  (bind _controllerreference (Variables|Default|GetControllerReference))
  ;[1 1 1] Apply User setting when game begins
  (Variables|/Game/Blueprints/Time_trial_blueprints/MainPlayerController.MainPlayerController_C|SetMaxLaps _controllerreference (Variables|CustomSettings|GetMaxLaps))
  (Variables|/Game/Blueprints/Time_trial_blueprints/MainPlayerController.MainPlayerController_C|SetSaveGameSlot _controllerreference (Variables|CustomSettings|GetSaveGameName))
  (CallFunction|UpdateTimes)
  (Default|StartGameSetup _controllerreference))

(event Custom|StartSequence
  (bind _checkpoints (Variables|Checkpoints|GetCheckpoints))
  ;[1 1 1] Initialising & activating Checkpoints
  (for (_array_element _array_index) (Variables|Checkpoints|GetCheckpoints)
    (Variables|/Game/Blueprints/Time_trial_blueprints/Checkpoint.Checkpoint_C|SetCheckpointNumber _array_element (+ _array_index 1))
    (Variables|Default|SetTotalCheckpoints (Utilities|Array|Length _checkpoints))
    (CallFunction|ActivateCheckpoint (Utilities|Array|Get(acopy) _checkpoints))
    (for _array_element_2 (Variables|Checkpoints|GetCheckpoints)
      (EventDispatchers|AssignCheckpointCleared _array_element_2 (delegate Custom|CheckCheckpointCleared)))))

(event Custom|CheckCheckpointCleared
  (params (NextCheckpoint :type Integer))
  (bind _controllerreference (Variables|Default|GetControllerReference))
  ;[1 1 1] Check to see if race is over, and restart if it is
  (CallFunction|LapCheck NextCheckpoint)
  (if (Variables|/Game/Blueprints/Time_trial_blueprints/MainPlayerController.MainPlayerController_C|GetRaceComplete _controllerreference)
    (Default|Restart _controllerreference)))

(event EventBeginPlay
  (bind _asmain_player_controller (Utilities|Casting|CastToMainPlayerController (Game|GetPlayerController 0)))
  (Variables|Default|SetControllerReference _asmain_player_controller)
  (CallFunction|ApplySettings)
  (CallFunction|StartSequence))

(fn ConstructionScript)

(fn UpdateTimes
  (bind _controllerreference (Variables|Default|GetControllerReference))
  ;[1 1 1] Pass the user times to MainPlayerController
  (Variables|/Game/Blueprints/Time_trial_blueprints/MainPlayerController.MainPlayerController_C|SetDefaultBestTotalTime _controllerreference (Variables|CustomSettings|GetDefaultBestTotal))
  (Variables|/Game/Blueprints/Time_trial_blueprints/MainPlayerController.MainPlayerController_C|SetDefaultBestLapTime _controllerreference (Variables|CustomSettings|GetDefaultBestLap)))

(fn LapCheck
  (params (Checkpoint :type Integer))
  ;[1 1 1] Checks to see if we've completed the race, or a lap, and sets up the next checkpoint
  (bind _output_get (LocalVariables|SetLocalCheckpoint Checkpoint))
  (if (== _output_get (Variables|Default|GetTotalCheckpoints))
    (bind _isracecomplete (CallFunction|CheckRaceComplete))
    (if _isracecomplete
      _
      (else
        (CallFunction|ActivateCheckpoint (Utilities|Array|Get(acopy) (Variables|Checkpoints|GetCheckpoints)))))
    (Default|UpdateLap (Variables|Default|GetControllerReference))
    (else
      (CallFunction|ActivateCheckpoint (Utilities|Array|Get(acopy) (Variables|Checkpoints|GetCheckpoints) (LocalVariables|GetLocalCheckpoint)))))
  (Variables|/Game/Blueprints/Time_trial_blueprints/MainPlayerController.MainPlayerController_C|SetRespawnLocation (Variables|Default|GetControllerReference) (Transformation|GetActorTransform (Utilities|Array|Get(acopy) (Variables|Checkpoints|GetCheckpoints) (- (LocalVariables|GetLocalCheckpoint) 1)))))

(fn ActivateCheckpoint
  (params (NextCheckpoint :type Checkpoint%20Object%20Reference))
  (bind _trigger (Variables|/Game/Blueprints/Time_trial_blueprints/Checkpoint.Checkpoint_C|GetTrigger NextCheckpoint))
  ;[1 1 1] Activates the next checkpoint
  (Development|SetHiddeninGame _trigger false false)
  (Variables|/Script/Engine.PrimitiveComponent|SetbGenerateOverlapEvents _trigger true))

(fn CheckRaceComplete
  (bind _controllerreference (Variables|Default|GetControllerReference))
  (bind _controllerreference_2 (Variables|Default|GetControllerReference))
  ;[1 1 1] Sets race to complete in MainPlayerController
  (if (>= (Variables|/Game/Blueprints/Time_trial_blueprints/MainPlayerController.MainPlayerController_C|GetActualLap _controllerreference) (Variables|/Game/Blueprints/Time_trial_blueprints/MainPlayerController.MainPlayerController_C|GetMaxLaps _controllerreference))
    (bind _output_get (Variables|/Game/Blueprints/Time_trial_blueprints/MainPlayerController.MainPlayerController_C|SetRaceComplete _controllerreference_2 true))
    (LocalVariables|SetLocalComplete _output_get)
    (else
      (bind _output_get_2 (Variables|/Game/Blueprints/Time_trial_blueprints/MainPlayerController.MainPlayerController_C|SetRaceComplete _controllerreference_2 false))
      (LocalVariables|SetLocalComplete _output_get_2)))
  (return (LocalVariables|GetLocalComplete)))

(fn GetTimeTrialTracker
  (return 0))