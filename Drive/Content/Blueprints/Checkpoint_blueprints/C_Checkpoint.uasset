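; Checkpoint actor for a timed vehicle race that clears itself when the player's vehicle drives through it.
; When a vehicle leaves the trigger, a dot product of its velocity and the arrow's forward vector accepts only forward passes.
; A valid pass fires the CheckpointCleared dispatcher with its checkpoint number, hides the trigger and particles, disables overlaps and adds time to the player controller's RemainingTime.
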(event OnComponentEndOverlap(Trigger)
  (params (OverlappedComponent :type Primitive%20Component%20Object%20Reference) (OtherActor :type Actor%20Object%20Reference) (OtherComp :type Primitive%20Component%20Object%20Reference) (OtherBodyIndex :type Integer))
  (bind _trigger (Variables|Default|GetTrigger))
  ;[1 1 1] Clearing checkpoints when vehicle pass through an updating the remaining time
  (bind _asvehicle_blueprint (Utilities|Casting|CastToVehicleBlueprint OtherActor))
  (if (> (Math|Vector|DotProduct (Transformation|GetVelocity _asvehicle_blueprint) (Math|Rotator|GetRotationXVector (Transformation|GetWorldRotation (Variables|Default|GetArrow)))) 0.0)
    (Default|CallCheckpointCleared (Variables|Default|GetCheckpointNumber))
    (Development|SetHiddeninGame _trigger true false)
    (Variables|/Script/Engine.PrimitiveComponent|SetbGenerateOverlapEvents _trigger false)
    (bind _asc_player_controller (Utilities|Casting|CastToC_PlayerController (Game|GetPlayerController 0)))
    (Variables|/Game/Blueprints/Checkpoint_blueprints/C_PlayerController.C_PlayerController_C|SetRemainingTime _asc_player_controller (+ (Variables|/Game/Blueprints/Checkpoint_blueprints/C_PlayerController.C_PlayerController_C|GetRemainingTime _asc_player_controller) 5.0))))

(fn ConstructionScript)